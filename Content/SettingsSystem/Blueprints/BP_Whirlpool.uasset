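; BP_Whirlpool is a one-shot Niagara effect actor that responds when the player character overlaps it.
; Two box triggers handle the two character types: Box casts to the third-person character and Box1 to the first-person one.
; Each has its own DoOnce, which plays that character's EffectSound, hides the Niagara effect, waits briefly, then destroys the actor.
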(event OnComponentBeginOverlap(Box)
  (params (OverlappedComponent :type Primitive%20Component%20Object%20Reference) (OtherActor :type Actor%20Object%20Reference) (OtherComp :type Primitive%20Component%20Object%20Reference) (OtherBodyIndex :type Integer) (bFromSweep :type Boolean) (SweepResult :type Hit%20Result%20Structure%20%28by%20ref%29))
  ;[1 1 1] Play Sound When Overlap Third Person Character
  (bind _asbp_third_person_character (Utilities|Casting|CastToBP_ThirdPersonCharacter OtherActor))
  (Utilities|FlowControl|DoOnce false
    (:Completed
      (Audio|Components|Audio|Play (Variables|/Game/SettingsSystem/DemoContent/ThirdPerson/Blueprints/BP_ThirdPersonCharacter.BP_ThirdPersonCharacter_C|GetEffectSound _asbp_third_person_character) 0.0)
      (Rendering|SetVisibility (Variables|Default|GetNiagara) false false)
      (Utilities|FlowControl|Delay 2.0)
      (Actor|DestroyActor))))

(event OnComponentBeginOverlap(Box1)
  (params (OverlappedComponent :type Primitive%20Component%20Object%20Reference) (OtherActor :type Actor%20Object%20Reference) (OtherComp :type Primitive%20Component%20Object%20Reference) (OtherBodyIndex :type Integer) (bFromSweep :type Boolean) (SweepResult :type Hit%20Result%20Structure%20%28by%20ref%29))
  ;[1 1 1] Play Sound When Overlap First Person Character
  (bind _asbp_first_person_character (Utilities|Casting|CastToBP_FirstPersonCharacter OtherActor))
  (Utilities|FlowControl|DoOnce false
    (:Completed
      (Audio|Components|Audio|Play (Variables|/Game/SettingsSystem/DemoContent/FirstPerson/BP_FirstPersonCharacter.BP_FirstPersonCharacter_C|GetEffectSound _asbp_first_person_character) 0.0)
      (Rendering|SetVisibility (Variables|Default|GetNiagara) false false)
      (Utilities|FlowControl|Delay 2.0)
      (Actor|DestroyActor))))

(fn ConstructionScript)