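; Game mode for a timed checkpoint race with a vehicle pawn, running a start countdown, a time limit and win/lose endings.
; BeginPlay binds finish-line and regular BP_Checkpoint crossing events, then holds input until the countdown ends and starts the lose timer.
; Winning clears the timer; either outcome shows its screen, disables input and handbrakes the car.
; Checkpoint time bonuses route to AddTimeToTimer, which is empty here.
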(event Custom|Game%20Start
  (Development|PrintString "Gejm started")
  (bind _returnvalue (Utilities|Time|SetTimerbyEvent (delegate Custom|Lose_OutofTime) (Variables|Default|GetStartTimerDuration)))
  (Variables|Default|SetTimeRemaniningTimer _returnvalue))

(event Custom|Game%20Finish
  (params (Win :type Boolean))
  (bind _returnvalue (Game|Player|GetPlayerPawn 0))
  (Development|PrintString (Utilities|String|SelectString "You Win" "You lose" Win))
  (Input|DisableInput _returnvalue (Game|GetPlayerController 0))
  (bind _asvehicle_adv_pawn (Utilities|Casting|CastToVehicleAdvPawn _returnvalue))
  (Class|ChaosVehicleMovementComponent|SetThrottleInput (Variables|/Script/ChaosVehicles.WheeledVehiclePawn|GetVehicleMovementComponent _asvehicle_adv_pawn) 0.0)
  (Class|ChaosVehicleMovementComponent|SetHandbrakeInput (Variables|/Script/ChaosVehicles.WheeledVehiclePawn|GetVehicleMovementComponent _asvehicle_adv_pawn) true)
  (Class|ChaosVehicleMovementComponent|SetSteeringInput (Variables|/Script/ChaosVehicles.WheeledVehiclePawn|GetVehicleMovementComponent _asvehicle_adv_pawn) 1.0))

(event Custom|Start%20Countdown)

(event Custom|Game%20Finish
  (params (Win :type Boolean)))

(event Custom|Start%20Countdown
  (bind _startcountdown_duration (Variables|Default|GetStartCountdown%20Duration))
  (Input|DisableInput (Game|Player|GetPlayerPawn 0) 0)
  (Development|PrintString "Countdown Started")
  (Utilities|FlowControl|Delay _startcountdown_duration)
  (Development|PrintText "Go" true true "(R=0.000000,G=0.660000,B=1.000000,A=1.000000)" _startcountdown_duration)
  (Input|EnableInput (Game|Player|GetPlayerPawn 0) 0)
  (CallFunction|GameStart))

(event Custom|Lose_OutofTime
  (bind _returnvalue (UserInterface|CreateWidget "/Game/RacingGame/Interfaces/LoseScreen.LoseScreen_C"))
  (UserInterface|Viewport|AddtoViewport _returnvalue 0)
  (Input|SetInputModeGameandUI (Game|GetPlayerController 0) (Variables|/Game/RacingGame/Interfaces/LoseScreen.LoseScreen_C|GetButton_0 _returnvalue) "DoNotLock" true false)
  (Variables|/Script/Engine.PlayerController|SetbShowMouseCursor (Game|GetPlayerController 0) true)
  (CallFunction|GameFinish false))

(event Custom|Win_CrossTheFinnishLine
  (Utilities|Time|ClearandInvalidateTimerbyHandle (Variables|Default|GetTimeRemaniningTimer))
  (bind _returnvalue (UserInterface|CreateWidget "/Game/RacingGame/Interfaces/WinScreen.WinScreen_C"))
  (UserInterface|Viewport|AddtoViewport _returnvalue 0)
  (Input|SetInputModeGameandUI (Game|GetPlayerController 0) (Variables|/Game/RacingGame/Interfaces/WinScreen.WinScreen_C|GetButton_0 _returnvalue) "DoNotLock" true false)
  (Variables|/Script/Engine.PlayerController|SetbShowMouseCursor (Game|GetPlayerController 0) true)
  (CallFunction|GameFinish true))

(event Custom|CrossedACheckpoint
  (params (TimeToAdd :type Integer))
  (CallFunction|AddTimetoTimer TimeToAdd))

(event EventBeginPlay
  (Utilities|FlowControl|Sequence
    (:then_0
      (bind _outactors (Actor|GetAllActorsOfClass "/Game/RacingGame/Checkpoints/BP_Checkpoint.BP_Checkpoint_C"))
      (for _array_element _outactors
        (if (Variables|/Game/RacingGame/Checkpoints/BP_Checkpoint.BP_Checkpoint_C|GetIsFinishLine _array_element)
          (EventDispatchers|BindEventtoOnCheckpointCrossed _array_element (EventDispatchers|CreateEvent :!event Custom|Win_CrossTheFinnishLine))
          (else
            (EventDispatchers|BindEventtoOnCheckpointCrossedwithTime _array_element (EventDispatchers|CreateEvent :!event Custom|CrossedACheckpoint))))))
    (:then_1
      (CallFunction|StartCountdown))))

(event EventTick
  (params (DeltaSeconds :type Float%20%28single-precision%29)))

(fn ConstructionScript)

(fn GameStart)

(fn AddTimetoTimer
  (params (TimeToAdd :type Integer)))